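; BP_GMTKInstance acts as the registry for BP_Link actors that connect pairs of objects.
; NewLink spawns and initializes a link at the source actor, unless that pair is already linked.
; Each link is stored in LinkMap under joined object-name keys for both directions, making lookup order-independent, and once in LinkSet.
; CollapseAll iterates LinkSet to collapse every registered link.
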(fn `CollapseAll`
  (bind _result (`BlueprintSetLibrary.Set_ToArray` (`self.LinkSet`)))
  (for _array_element _result
    (`/Game/Assets/BP/BP_Link.CollapseLink` _array_element)))

(fn `NewLink`
  (params (From :type "/Game/Assets/BP/BP_Block Object Reference") (To :type "/Game/Assets/BP/BP_Block Object Reference"))
  (returns (CreatedLink :type "/Game/Assets/BP/BP_Link Object Reference"))
  (locals (TheCreatedLink :type "/Game/Assets/BP/BP_Link Object Reference"))
  (bind _returnvalue (`KismetSystemLibrary.GetObjectName` To))
  (bind _returnvalue_2 (`KismetSystemLibrary.GetObjectName` From))
  (bind _linkmap (`self.LinkMap`))
  (bind _returnvalue_3 (`KismetStringLibrary.JoinStringArray` (`|MakeArray` _returnvalue _returnvalue_2) "_"))
  (bind _returnvalue_4 (`KismetStringLibrary.JoinStringArray` (`|MakeArray` _returnvalue_2 _returnvalue) "_"))
  ;[1 1 1] Check if link already exists
  (if (not (or (`BlueprintMapLibrary.Map_Contains` _linkmap _returnvalue_4) (`BlueprintMapLibrary.Map_Contains` _linkmap _returnvalue_3)))
    (bind _returnvalue_5 (`|SpawnActorFromClass` "/Game/Assets/BP/BP_Link.BP_Link_C" (`Actor.GetTransform` From) "Undefined" "OverrideRootScale" null null))
    (`/Game/Assets/BP/BP_Link.CreateLink` _returnvalue_5 From To)
    (`BlueprintMapLibrary.Map_Add` _linkmap _returnvalue_4 _returnvalue_5)
    (`BlueprintMapLibrary.Map_Add` _linkmap _returnvalue_3 _returnvalue_5)
    (`BlueprintSetLibrary.Set_Add` (`self.LinkSet`) _returnvalue_5)
    (return _returnvalue_5)))