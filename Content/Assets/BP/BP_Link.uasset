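; BP_Link is an actor that represents a visual connection between two other actors, From and To.
; CreateLink stores the two endpoints, or destroys the link if they are the same or either is invalid.
; Each Tick, while both endpoints are valid, it draws a thick green debug line between their current locations, so the link follows them as they move.
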(event `self.ReceiveTick`
  (params (DeltaSeconds :type "Float (single-precision)"))
  (bind __from (`self._From`))
  (bind __to (`self._To`))
  ;[1 1 1] DisplayLink
  (if (and (`KismetSystemLibrary.IsValid` __from) (`KismetSystemLibrary.IsValid` __to))
    (`KismetSystemLibrary.DrawDebugLine` (`self.K2_GetActorLocation` __from) (`self.K2_GetActorLocation` __to) (struct :`G` 0.921875 :`B` 0.49011 :`A` 1.0) 0.0 8.0)))

(event `InputAction|Fire`
  (params (Key :type "Key Structure")))

(fn `CreateLink`
  (params (From :type "/Game/Assets/BP/BP_Block Object Reference") (To :type "/Game/Assets/BP/BP_Block Object Reference"))
  (if (and (not (== From To)) (`KismetSystemLibrary.IsValid` From) (`KismetSystemLibrary.IsValid` To))
    (set `self._From` From)
    (set `self._To` To)
    (else
      (`self.K2_DestroyActor`))))

(fn `UserConstructionScript`)